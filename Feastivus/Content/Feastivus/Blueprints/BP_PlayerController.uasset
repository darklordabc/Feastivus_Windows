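; Player controller for the Feastivus kitchen game that shows the current orders on screen.
; On begin play, the local controller creates an order list widget and adds it to the viewport.
; It then syncs by reading the orders from the kitchen game state and adding a widget to the list for each one.
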(event `self.ReceiveBeginPlay`
  (if (`self.IsLocalPlayerController`)
    (bind _returnvalue (`|CreateWidget` "/Game/Feastivus/Blueprints/Widgets/BPW_OrderList.BPW_OrderList_C" self))
    (bind _output_get (set `self.OrderList` _returnvalue))
    (`UserWidget.AddToViewport` _output_get 0)
    (`self.SyncOrders`)))

(fn `SyncOrders`
  (bind _asbp_game_state_kitchen_base (`/Game/Feastivus/Blueprints/BPML_FeastivusAPI.GetGameStateKitchen`)
    (:`then`
      (for _array_element (`/Game/Feastivus/Blueprints/BP_GameStateKitchenBase.Orders` _asbp_game_state_kitchen_base)
        (`/Game/Feastivus/Blueprints/Widgets/BPW_OrderList.AddOrderWidget` (`self.OrderList`) _array_element)))))

(fn `UserConstructionScript`)