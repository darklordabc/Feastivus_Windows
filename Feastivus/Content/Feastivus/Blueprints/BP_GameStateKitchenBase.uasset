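; Base game state for the Feastivus kitchen, scheduling timed customer orders and relaying them to players' order list UI.
; InitOrders steps through DT_Orders with a manually advanced loop, delaying until each row's cumulative Time before storing it in Orders.
; Multicast events add orders or set their success result on the local player controller's OrderList, skipping dedicated servers.
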(event `self.ReceiveBeginPlay`)

(event `self.ReceiveTick`
  (params (DeltaSeconds :type "Float (single-precision)")))

(event `InitOrders`
  (bind _outrownames (`DataTableFunctionLibrary.GetDataTableRowNames` "/Game/Feastivus/Recipes/DT_Orders.DT_Orders"))
  (bind _arrayelement (`/Game/Feastivus/Blueprints/BPML_FeastivusAPI.ForEachLoopAlternate` _outrownames :!label _label)
    (:`Loop Body`
      (bind _returnvalue (`|GetDataTableRow` "/Game/Feastivus/Recipes/DT_Orders.DT_Orders" _arrayelement)
        (:`then`
          (bind _returnvalue_2 (- (`.Time_6_26B30E474B7E488E6AC79390B581214A` (break `/Game/Feastivus/Recipes/S_Order` _returnvalue)) (`self.OrderTimer`)))
          (`KismetSystemLibrary.Delay` _returnvalue_2)
          (set `self.OrderTimer` (+ _returnvalue_2 (`self.OrderTimer`)))
          (`KismetArrayLibrary.Array_Add` (`self.Orders`) _returnvalue)
          (`self.MulticastAddOrderWidget` _returnvalue)
          (goto _label :!via `NextBody`))))))

(event `MulticastAddOrderWidget`
  (params (Order :type "/Game/Feastivus/Recipes/S_Order Structure"))
  (`/Game/Feastivus/Blueprints/BPML_FeastivusAPI.SwitchIsDedicatedServer`
    (:`false`
      (bind _asbp_player_controller (cast `/Game/Feastivus/Blueprints/BP_PlayerController` (`GameplayStatics.GetPlayerController` 0)))
      (`/Game/Feastivus/Blueprints/Widgets/BPW_OrderList.AddOrder` (`/Game/Feastivus/Blueprints/BP_PlayerController.OrderList` _asbp_player_controller) Order))))

(event `MulticastSetOrderWidgetResult`
  (params (Index :type Integer) (bSuccess :type Boolean))
  (`/Game/Feastivus/Blueprints/BPML_FeastivusAPI.SwitchIsDedicatedServer`
    (:`false`
      (bind _asbp_player_controller (cast `/Game/Feastivus/Blueprints/BP_PlayerController` (`GameplayStatics.GetPlayerController` 0)))
      (`/Game/Feastivus/Blueprints/Widgets/BPW_OrderList.SetOrderResult` (`/Game/Feastivus/Blueprints/BP_PlayerController.OrderList` _asbp_player_controller) Index bSuccess))))

(fn `UserConstructionScript`)