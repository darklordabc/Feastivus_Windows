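; Base game mode for kitchen levels in Feastivus, handling order startup, recipe data and player spawn selection.
; When the match state changes to InProgress, it tells the kitchen game state to initialize orders.
; GetRecipes builds a recipe list from the class defaults of its configured Dishes.
; ChoosePlayerStart gives players successive spawn points by matching each PlayerStart tag to an incrementing index.
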(event `self.K2_OnSetMatchState`
  (params (NewState :type Name))
  (if (== NewState "InProgress")
    (bind _asbp_game_state_kitchen_base (`/Game/Feastivus/Blueprints/BPML_FeastivusAPI.GetGameStateKitchen`)
      (:`then`
        (`/Game/Feastivus/Blueprints/BP_GameStateKitchenBase.InitOrders` _asbp_game_state_kitchen_base)))))

(event `self.ReceiveBeginPlay`)

(event `self.ReceiveTick`
  (params (DeltaSeconds :type "Float (single-precision)")))

(fn `ChoosePlayerStart`
  (params (Player :type "Controller Object Reference"))
  (returns (ReturnValue :type "Actor Object Reference"))
  (bind _outactors (`GameplayStatics.GetAllActorsOfClass` "/Script/Engine.PlayerStart"))
  (for _array_element _outactors
    (if (== (`PlayerStart.PlayerStartTag` _array_element) (`KismetStringLibrary.Conv_StringToName` (`KismetStringLibrary.Conv_IntToString` (`self.PlayerStartIndex`))))
      (`/Engine/EditorBlueprintResources/StandardMacros.IncrementInt` (`self.PlayerStartIndex`)
        (:`  `
          (return _array_element))))))

(fn `GetRecipes`
  (returns (Recipes :type "Array of Recipe Structure"))
  (locals (RecipesLocal :type "Array of Recipe Structure"))
  (for _array_element (`self.Dishes`)
    (`KismetArrayLibrary.Array_Add` (`local.RecipesLocal`) (defaults `/Game/Feastivus/Blueprints/BP_GameModeKitchenBase` _array_element)))
  (return (`local.RecipesLocal`)))

(fn `UserConstructionScript`)