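; BP_Camera is a shared camera actor that follows the midpoint of all players in Feastivus.
; On Tick, only when not running as server, it gathers every BP_Player and averages their locations.
; It eases toward that average's X and Y with VInterpTo, while targeting the height stored in ZLocation.
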(event `self.ReceiveBeginPlay`)

(event `self.ReceiveTick`
  (params (DeltaSeconds :type "Float (single-precision)"))
  (if (not (`KismetSystemLibrary.IsServer`))
    (bind _outactors (`GameplayStatics.GetAllActorsOfClass` "/Game/Feastivus/Blueprints/Gameplay/BP_Player.BP_Player_C"))
    (set `self.Middle` (0.0 0.0 0.0))
    (for _array_element _outactors
      (set `self.Middle` (+ (`self.Middle`) (`self.K2_GetActorLocation` _array_element))))
    (bind (_returnvalue_x _returnvalue_y) (`KismetMathLibrary.BreakVector` (/ (`self.Middle`) (`KismetArrayLibrary.Array_Length` _outactors))))
    (`self.K2_SetActorLocation` (`KismetMathLibrary.VInterpTo` (`self.K2_GetActorLocation`) (`KismetMathLibrary.MakeVector` _returnvalue_x _returnvalue_y (`self.ZLocation`)) (* DeltaSeconds 1.0) 4.0))))

(fn `UserConstructionScript`)