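; BP_ConveyorChain builds and manages a chain of BP_Conveyor bench actors along a path.
; Four directional Add functions feed SpawnConveyor, which places each conveyor 130 units beyond the last one's facing and rotates it toward the chosen direction.
; Each new conveyor links to its predecessor and any following conveyor through PreviousBench and FindNextBench, and references the chain.
; Helpers remove the last conveyor, clear the whole chain or return its end.
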(event `self.ReceiveBeginPlay`)

(fn `AddBottom`
  (`self.SpawnConveyor` (-130.0 0.0 0.0)))

(fn `AddLeft`
  (`self.SpawnConveyor` (0.0 -130.0 0.0)))

(fn `AddRight`
  (`self.SpawnConveyor` (0.0 130.0 0.0)))

(fn `AddUp`
  (`self.SpawnConveyor` (130.0 0.0 0.0)))

(fn `Clean`
  (`/Game/Feastivus/Blueprints/BPFL_FeastivusAPI.DestroyArrayOfActors` (`self.Conveyors`))
  (`KismetArrayLibrary.Array_Clear` (`self.Conveyors`)))

(fn `GetLastConveyor`
  (returns (`Last Conveyor` :type "/Game/Feastivus/Blueprints/Gameplay/Benches/BP_Conveyor Object Reference"))
  (bind _conveyors (`self.Conveyors`))
  (return (`|GetArrayItem` _conveyors (`KismetArrayLibrary.Array_LastIndex` _conveyors))))

(fn `RemoveLast`
  (bind _returnvalue (`KismetArrayLibrary.Array_LastIndex` (`self.Conveyors`)))
  (`/Game/Feastivus/Blueprints/BPFL_FeastivusAPI.DestroyActorAndAttachedActors` (`|GetArrayItem` (`self.Conveyors`) _returnvalue))
  (`KismetArrayLibrary.Array_Remove` (`self.Conveyors`) _returnvalue))

(fn `SpawnConveyor`
  (params (LocationOffset :type "Vector Structure"))
  (locals (Origin :type "Vector Structure"))
  (bind _origin (`local.Origin`))
  (bind _conveyors (`self.Conveyors`))
  (bind _output (`|GetArrayItem` (`self.Conveyors`) (`KismetArrayLibrary.Array_LastIndex` (`self.Conveyors`))))
  (bind _output_2 (`|GetArrayItem` _conveyors (`KismetArrayLibrary.Array_LastIndex` _conveyors)))
  (if (== (`KismetArrayLibrary.Array_Length` (`self.Conveyors`)) 0)
    (set `local.Origin` (`self.K2_GetActorLocation`))
    (else
      (set `local.Origin` (+ (`self.K2_GetActorLocation` _output) (* (`KismetMathLibrary.Conv_RotatorToVector` (`self.K2_GetActorRotation` _output)) 130.0)))))
  (bind _returnvalue (`|SpawnActorFromClass` "/Game/Feastivus/Blueprints/Gameplay/Benches/BP_Conveyor.BP_Conveyor_C" (`KismetMathLibrary.MakeTransform` _origin) "Undefined" "OverrideRootScale" null null))
  (`self.K2_SetActorRotation` _returnvalue (`KismetMathLibrary.Conv_VectorToRotator` (`KismetMathLibrary.GetDirectionUnitVector` _origin (+ (`local.Origin`) (`local.LocationOffset`)))) false)
  (set `/Game/Feastivus/Blueprints/Gameplay/Benches/BP_Conveyor.PreviousBench` _output_2 _returnvalue)
  (`/Game/Feastivus/Blueprints/Gameplay/Benches/BP_Conveyor.FindNextBench` _output_2)
  (bind _asbp_table (`/Game/Feastivus/Blueprints/Gameplay/Benches/BP_Conveyor.FindNextBench` _returnvalue))
  (bind _asbp_conveyor (cast `/Game/Feastivus/Blueprints/Gameplay/Benches/BP_Conveyor` _asbp_table)
    (:`then`
      (set `/Game/Feastivus/Blueprints/Gameplay/Benches/BP_Conveyor.PreviousBench` _returnvalue _asbp_conveyor))
    (:`CastFailed`
      _))
  (set `/Game/Feastivus/Blueprints/Gameplay/Benches/BP_Conveyor.Chain` self _returnvalue)
  (`KismetArrayLibrary.Array_Add` (`self.Conveyors`) _returnvalue)
  (return))

(fn `UserConstructionScript`)