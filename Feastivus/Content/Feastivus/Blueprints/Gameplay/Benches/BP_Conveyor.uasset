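; Conveyor bench that players place items on or take from, carrying them along a chain of conveyors toward a table.
; On the server, Tick advances a looping time and moves items along a straight or CurveVector path, chosen by comparing rotation with the previous bench.
; Items pass to the next bench found by a forward trace, with MovementInflictor tracking the owning conveyor.
; Movement halts while the table ending the chain is occupied.
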(event `self.ReceiveBeginPlay`
  (`parent.ReceiveBeginPlay`))

(event `self.ReceiveTick`
  (params (DeltaSeconds :type "Float (single-precision)"))
  (bind _nextbench (`self.NextBench`))
  (bind _newobjects (`/Game/Feastivus/Blueprints/Gameplay/Benches/BP_ConveyorChain.NewObjects` (`self.Chain`)))
  (bind _nextbench_2 (`/Game/Feastivus/Blueprints/Gameplay/Benches/BP_Conveyor.NextBench` (`/Game/Feastivus/Blueprints/Gameplay/Benches/BP_ConveyorChain.GetLastConveyor` (`self.Chain`))))
  (`parent.ReceiveTick` DeltaSeconds)
  (`/Engine/EditorBlueprintResources/ActorMacros.Switch Has Authority`
    (:`Authority`
      (set `self.CurrentTime` (`KismetMathLibrary.FClamp` (+ (`self.CurrentTime`) (* 1.0 (`self.Speed`)))))
      (if true
        (`/Game/Feastivus/Blueprints/BPML_FeastivusAPI.IsObjectChildOf` _nextbench_2 "BP_Conveyor_C"
          (:`True`
            (bind _asbp_conveyor (cast `/Game/Feastivus/Blueprints/Gameplay/Benches/BP_Conveyor` (`self.NextBench`) :!label _label)
              (:`then`
                (bind _bmoving (`self.IsEmpty` _asbp_conveyor))
                (if _bmoving
                  _
                  (else
                    _)))
              (:`CastFailed`
                _))
            (bind _keys (`BlueprintMapLibrary.Map_Keys` (`self.ObjectState`)))
            (for _array_element _keys
              (if (`BlueprintMapLibrary.Map_Contains` (`self.ObjectState`) _array_element)
                (`/Engine/EditorBlueprintResources/StandardMacros.IsValid` (`self.GetAttachParentActor` _array_element)
                  (:`Is Not Valid`
                    (bind _asbp_dynamic_object (cast `/Game/Feastivus/Blueprints/Gameplay/BP_DynamicObject` _array_element :!pure true))
                    (bind _movementinflictor (`/Game/Feastivus/Blueprints/Gameplay/BP_DynamicObject.MovementInflictor` _asbp_dynamic_object))
                    (`/Engine/EditorBlueprintResources/StandardMacros.IsValid` _movementinflictor
                      (:`Is Valid`
                        (if (== _movementinflictor self)
                          (bind _location (`self.GetConveyorObjectLocation` 1.0 :!label _label_2))
                          (if (< (`KismetMathLibrary.VSizeXY` (- _location (`self.K2_GetActorLocation` _array_element))) 0.01)
                            (if (`BlueprintMapLibrary.Map_Find` (`self.ObjectState`) _asbp_dynamic_object)
                              (`/Game/Feastivus/Blueprints/BPML_FeastivusAPI.IsObjectChildOf` _nextbench "BP_Conveyor_C"
                                (:`True`
                                  (set `/Game/Feastivus/Blueprints/Gameplay/BP_DynamicObject.MovementInflictor` _nextbench _asbp_dynamic_object)
                                  (`BlueprintMapLibrary.Map_Remove` (`self.ObjectState`) _asbp_dynamic_object)
                                  (`BlueprintMapLibrary.Map_Add` (`/Game/Feastivus/Blueprints/Gameplay/Benches/BP_Conveyor.ObjectState` (cast `/Game/Feastivus/Blueprints/Gameplay/Benches/BP_Conveyor` _nextbench :!pure true)) _asbp_dynamic_object))
                                (:`False`
                                  (bind _asbp_table (cast `/Game/Feastivus/Blueprints/Gameplay/Benches/BP_Table` (`self.NextBench`)))
                                  (`/Game/Feastivus/Blueprints/Gameplay/Benches/BP_Table.SetHoldingObject` _asbp_table (cast `/Game/Feastivus/Blueprints/Gameplay/BP_DynamicObject` _array_element :!pure true))))
                              (else
                                (`BlueprintMapLibrary.Map_Add` (`self.ObjectState`) _asbp_dynamic_object true)
                                (if (`KismetArrayLibrary.Array_Contains` _newobjects _asbp_dynamic_object)
                                  (`KismetArrayLibrary.Array_RemoveItem` _newobjects _asbp_dynamic_object))))
                            (else
                              (bind _location_2 (`self.GetConveyorObjectLocation` (`self.CurrentTime`)))
                              (`self.K2_SetActorLocation` _array_element _location_2 false false)))))
                      (:`Is Not Valid`
                        (set `/Game/Feastivus/Blueprints/Gameplay/BP_DynamicObject.MovementInflictor` self _asbp_dynamic_object)
                        (goto _label_2)))))))
            (if (== (`self.CurrentTime`) 1.0)
              (set `self.CurrentTime` 0.0)))
          (:`False`
            (bind _asbp_table_2 (cast `/Game/Feastivus/Blueprints/Gameplay/Benches/BP_Table` _nextbench_2))
            (bind _free (`/Game/Feastivus/Blueprints/Gameplay/Benches/BP_Table.IsFree` _asbp_table_2))
            (if _free
              (goto _label))))))))

(fn `FindBench`
  (params (Location :type "Vector Structure"))
  (returns (Actor :type "Actor Object Reference"))
  (bind (_outhit _returnvalue) (`KismetSystemLibrary.LineTraceSingle` :`Start` (+ Location (0.0 0.0 500.0)) :`End` Location :`TraceChannel` "TraceTypeQuery1" :`DrawTime` 10.0))
  (if _returnvalue
    (return (`.HitActor` (`GameplayStatics.BreakHitResult` _outhit)))
    (else
      (return null))))

(fn `FindNextBench`
  (returns (`AsBP Table` :type "/Game/Feastivus/Blueprints/Gameplay/BP_StaticObject Object Reference"))
  (bind _actor (`self.FindBench` (+ (`self.K2_GetActorLocation`) (* (`KismetMathLibrary.Conv_RotatorToVector` (`self.K2_GetActorRotation`)) 130.0))))
  (bind _asbp_static_object (cast `/Game/Feastivus/Blueprints/Gameplay/BP_StaticObject` _actor)
    (:`then`
      (bind _output_get (set `self.NextBench` _asbp_static_object)))
    (:`CastFailed`
      _))
  (return _output_get))

(fn `GetConveyorObjectLocation`
  (params (Time :type "Float (double-precision)"))
  (returns (Location :type "Vector Structure"))
  (locals (LocationLocal :type "Vector Structure" :default (0.0 0.0 0.0)) (CurveVector :type "CurveVector Object Reference" :default "CurveVector'/Game/Feastivus/Blueprints/Gameplay/Benches/C_Conveyor.C_Conveyor'"))
  (bind (_returnvalue_x _returnvalue_y _returnvalue_z) (`KismetMathLibrary.BreakVector` (`self.K2_GetActorLocation`)))
  (bind _location (`self.GetConveyorObjectRelativeLocation` Time))
  (bind (_returnvalue_x_2 _returnvalue_y_2) (`KismetMathLibrary.BreakVector` (`KismetMathLibrary.TransformLocation` (`self.GetTransform`) _location)))
  (return (`KismetMathLibrary.MakeVector` _returnvalue_x_2 _returnvalue_y_2 (+ _returnvalue_z 85.0))))

(fn `GetConveyorObjectRelativeLocation`
  (params (Time :type "Float (double-precision)"))
  (returns (Location :type "Vector Structure"))
  (locals (LocationLocal :type "Vector Structure" :default (0.0 0.0 0.0)) (CurveVector :type "CurveVector Object Reference" :default "CurveVector'/Game/Feastivus/Blueprints/Gameplay/Benches/C_Conveyor.C_Conveyor'"))
  (if (== (`self.K2_GetActorRotation`) (`self.K2_GetActorRotation` (`self.PreviousBench`)) :`ErrorTolerance` 1.0)
    (bind _output_get (set `local.LocationLocal` (`KismetMathLibrary.MakeVector` (- (* Time 130.0) 65.0))))
    (return _output_get)
    (else
      (bind _output_get_2 (set `local.LocationLocal` (`KismetMathLibrary.RotateAngleAxis` (`CurveVector.GetVectorValue` (`local.CurveVector`) (`local.Time`)) 180.0 (0.0 0.0 1.0))))
      (return _output_get_2))))

(fn `InteractWith`
  (params (Object :type "/Game/Feastivus/Blueprints/Gameplay/BP_DynamicObject Object Reference") (Player :type "/Game/Feastivus/Blueprints/Gameplay/BP_Player Object Reference"))
  (returns (bStartProcessing :type Boolean) (bSuccess :type Boolean))
  (`/Engine/EditorBlueprintResources/StandardMacros.IsValid` Object
    (:`Is Valid`
      (if (== (`BlueprintMapLibrary.Map_Length` (`self.ObjectState`)) 0)
        (bind _object (`/Game/Feastivus/Blueprints/Gameplay/BP_Player.FreeHoldingObject` Player))
        (`BlueprintMapLibrary.Map_Add` (`self.ObjectState`) _object)
        (`self.SetActorEnableCollision` _object false)
        (`KismetArrayLibrary.Array_AddUnique` (`/Game/Feastivus/Blueprints/Gameplay/Benches/BP_ConveyorChain.NewObjects` (`self.Chain`)) _object)
        (bind _location (`self.GetConveyorObjectLocation` 0.5))
        (`self.K2_SetActorLocation` _object _location false false)
        (return false true)
        (else
          (return false false))))
    (:`Is Not Valid`
      (bind _keys (`BlueprintMapLibrary.Map_Keys` (`self.ObjectState`)))
      (bind _output (`|GetArrayItem` _keys))
      (`/Engine/EditorBlueprintResources/StandardMacros.IsValid` _output
        (:`Is Valid`
          (bind _asbp_dynamic_object (cast `/Game/Feastivus/Blueprints/Gameplay/BP_DynamicObject` _output))
          (`/Game/Feastivus/Blueprints/Gameplay/BP_Player.SetHoldingObject` Player _asbp_dynamic_object)
          (`self.SetActorEnableCollision` _asbp_dynamic_object true)
          (`BlueprintMapLibrary.Map_Remove` (`self.ObjectState`) _asbp_dynamic_object)
          (`KismetArrayLibrary.Array_RemoveItem` (`/Game/Feastivus/Blueprints/Gameplay/Benches/BP_ConveyorChain.NewObjects` (`self.Chain`)) _asbp_dynamic_object))))))

(fn `IsEmpty`
  (returns (bMoving :type Boolean))
  (return (== (`BlueprintMapLibrary.Map_Length` (`self.ObjectState`)) 0)))

(fn `UserConstructionScript`
  (`parent.UserConstructionScript`))