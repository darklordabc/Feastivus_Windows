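; BP_Masher is a processing bench that mashes targets into a result item.
; It accepts a new user and target only when it has no targets or the new target matches the class of the first, then defers to the parent.
; When processing finishes, it reads the mashing message from the first target before calling the parent finish logic, then spawns the result from that message and holds it.
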(event `self.OnProcessingFinished`
  (bind _target (message `/Game/Feastivus/Blueprints/Gameplay/Ingredients/BPI_Mashable.GetMashingTarget` (`|GetArrayItem` (`self.Targets`))))
  (`parent.OnProcessingFinished`)
  (bind _spawnedobject (`self.SpawnProcessingResult` _target))
  (`/Game/Feastivus/Blueprints/Gameplay/BPI_ObjectHolder.SetHoldingObject` _spawnedobject))

(fn `AddUserAndTarget`
  (params (User :type "/Game/Feastivus/Blueprints/Gameplay/BP_Player Object Reference") (Target :type "/Game/Feastivus/Blueprints/Gameplay/BP_DynamicObject Object Reference"))
  (returns (bSuccess :type Boolean))
  (if (> (`KismetArrayLibrary.Array_Length` (`self.Targets`)) 0)
    (if (== (`GameplayStatics.GetObjectClass` (`|GetArrayItem` (`self.Targets`))) (`GameplayStatics.GetObjectClass` Target))
      _
      (else
        (return false))))
  (bind _bsuccess (`parent.AddUserAndTarget` (`local.User`) (`local.Target`)))
  (return _bsuccess))

(fn `UserConstructionScript`
  (`parent.UserConstructionScript`))