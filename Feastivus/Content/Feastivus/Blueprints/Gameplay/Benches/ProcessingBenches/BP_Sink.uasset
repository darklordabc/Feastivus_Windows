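; BP_Sink is a processing bench that turns washable items, single or stacked, into their washed results.
; When processing finishes, it asks the target, or a stack's first object, for the result class via GetWashingTargetMessage.
; A stack yields one result per object, all of that same class, in a newly spawned pickable BP_Stack.
; After calling the parent's finish logic, the bench holds the new stack or single result.
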(fn `OnProcessingFinished`
  (locals (NewStackObjects :type "Array of /Game/Feastivus/Blueprints/Gameplay/BP_DynamicObject Object Reference") (ResultClass :type "/Game/Feastivus/Blueprints/Gameplay/BP_DynamicObject Class Reference"))
  (bind _output (`|GetArrayItem` (`self.Targets`)))
  (`/Game/Feastivus/Blueprints/BPML_FeastivusAPI.IsObjectChildOf` _output "/Game/Feastivus/Blueprints/Gameplay/Tools/BP_Stack.BP_Stack_C"
    (:`True`
      (bind _asbp_stack (cast `/Game/Feastivus/Blueprints/Gameplay/Tools/BP_Stack` (`|GetArrayItem` (`self.Targets`))))
      (bind _objects (`/Game/Feastivus/Blueprints/Gameplay/Tools/BP_Stack.Objects` _asbp_stack))
      (bind _washingtarget (message `/Game/Feastivus/Blueprints/Gameplay/Tools/BPI_Washable.GetWashingTarget` (`|GetArrayItem` _objects)))
      (for _ (range (+ (`KismetArrayLibrary.Array_LastIndex` _objects) 1))
        (bind _spawnedobject (`self.SpawnProcessingResult` _washingtarget))
        (`KismetArrayLibrary.Array_Add` (`local.NewStackObjects`) _spawnedobject))
      (bind _returnvalue (`|SpawnActorFromClass` "/Game/Feastivus/Blueprints/Gameplay/Tools/BP_Stack.BP_Stack_C" (`KismetMathLibrary.MakeTransform` (0.0 0.0 0.0)) "AlwaysSpawn" "OverrideRootScale" null (`local.NewStackObjects`) true null))
      (`parent.OnProcessingFinished`)
      (`/Game/Feastivus/Blueprints/Gameplay/BPI_ObjectHolder.SetHoldingObject` _returnvalue)
      (return))
    (:`False`
      (bind _washingtarget_2 (message `/Game/Feastivus/Blueprints/Gameplay/Tools/BPI_Washable.GetWashingTarget` _output))
      (set `local.ResultClass` _washingtarget_2)
      (`parent.OnProcessingFinished`)
      (bind _spawnedobject_2 (`self.SpawnProcessingResult` (`local.ResultClass`)))
      (`/Game/Feastivus/Blueprints/Gameplay/BPI_ObjectHolder.SetHoldingObject` _spawnedobject_2)
      (return))))

(fn `UserConstructionScript`
  (`parent.UserConstructionScript`))