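; Processing bench where a player places an object implementing ProcessingTypeInterface to be worked on over time; other objects go through a swap.
; InteractWith runs on authority, binding user and target, then plays a timeline that drives a progress-bar widget with the target's icon.
; Interrupting releases the user but keeps target and timeline position, so a free-handed player can resume.
; Completion destroys the held object and resets the bench; a helper can spawn result actors.
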(event `self.ReceiveBeginPlay`
  (`parent.ReceiveBeginPlay`)
  (bind _asbpw_simple_progress_bar (`self.GetProgressWidget`))
  (`Widget.SetVisibility` _asbpw_simple_progress_bar "Hidden"))

(event `/Game/Feastivus/Blueprints/Gameplay/Benches/BPI_IngredientProcessor.StartProcessing`
  (`/Game/Feastivus/Blueprints/Gameplay/Benches/BPI_IngredientProcessor.StartProcessing`))

(event `Start Processing Routine`
  (`/Engine/EditorBlueprintResources/ActorMacros.Switch Has Authority`
    (:`Authority`
      (bind (_direction _loop) (`Timeline|ProcessingTimeline` :!label _label)
        (:`Update`
          (`self.Event Update Progress` _loop))
        (:`Finished`
          (`self.OnProcessingFinished`)
          (goto _label :!via `SetNewTime`))))))

(event `/Game/Feastivus/Blueprints/Gameplay/Benches/BPI_IngredientProcessor.InterruptProcessing`
  (`self.Interrupt Processing Routine`))

(event `Interrupt Processing Routine`
  (set `/Game/Feastivus/Blueprints/Gameplay/BP_Player.ProcessingBench` null (`self.CurrentUser`))
  (set `self.CurrentUser` null)
  (goto _label :!via `Stop`))

(event `Event Update Progress`
  (params (Progress :type "Float (double-precision)"))
  (bind _returnvalue (and (> Progress 0.0) (<= Progress 1.0)))
  (bind _asbpw_simple_progress_bar (`self.GetProgressWidget`))
  ;[1 0.3371 0.4269] TODO: Refactor this
  (`Widget.SetVisibility` _asbpw_simple_progress_bar (select `bool` _returnvalue :`false` "Hidden" :`true` "Visible" :!type "ESlateVisibility Enum"))
  (if _returnvalue
    (`/Game/Feastivus/Blueprints/Widgets/BPW_IconWithProgressBar.SetProgress` _asbpw_simple_progress_bar Progress)
    (bind _texture (`/Game/Feastivus/Blueprints/BPFL_FeastivusAPI.GetIconTexture` (`GameplayStatics.GetObjectClass` (`self.CurrentProcessingTarget`))))
    (set `/Game/Feastivus/Blueprints/Widgets/BPW_Icon.IconTexture` _texture (`/Game/Feastivus/Blueprints/Widgets/BPW_IconWithProgressBar.BPW_Icon` _asbpw_simple_progress_bar))))

(fn `AvailableToPickFrom`
  (returns (AvailableToPickFrom :type Boolean))
  (return (not (or (`KismetSystemLibrary.IsValid` (`self.CurrentUser`)) (`KismetSystemLibrary.IsValid` (`self.CurrentProcessingTarget`))))))

(fn `InteractWith`
  (params (Object :type "/Game/Feastivus/Blueprints/Gameplay/BP_DynamicObject Object Reference") (Player :type "/Game/Feastivus/Blueprints/Gameplay/BP_Player Object Reference"))
  (returns (bStartProcessing :type Boolean) (bSuccess :type Boolean))
  (`/Engine/EditorBlueprintResources/ActorMacros.Switch Has Authority`
    (:`Authority`
      (bind _availabletopickfrom (`self.AvailableToPickFrom`))
      (if _availabletopickfrom
        (bind _free (`/Game/Feastivus/Blueprints/Gameplay/BPI_ObjectHolder.IsFree`))
        (if _free
          (bind _processingtarget (`self.SetCurrentUserAndChoppingTarget` Object Player)
            (:`Success`
              (if (and (`KismetSystemLibrary.DoesImplementInterface` _processingtarget (`self.ProcessingTypeInterface`)) (`KismetSystemLibrary.IsValid` (`self.CurrentProcessingTarget`)))
                (set `/Game/Feastivus/Blueprints/Gameplay/BP_Player.HoldingObject` null (`self.CurrentUser`))
                (set `self.HoldingObject` (`self.CurrentProcessingTarget`))
                (set `/Game/Feastivus/Blueprints/Gameplay/BP_Player.ProcessingBench` self (`self.CurrentUser`) :!label _label)
                (`self.Start Processing Routine`)
                (return true true)
                (else
                  (`self.Event Swap Objects` (`self.CurrentProcessingTarget`) (`self.CurrentUser`))
                  (`self.ResetCurrentUserAndChoppingTarget`))))
            (:`Failed`
              (`self.Event Swap Objects` Object Player :!label _label_2)))
          (else
            (goto _label_2)))
        (else
          (bind _free_2 (`/Game/Feastivus/Blueprints/Gameplay/BP_Player.IsFree` Player))
          (if (and (not (`KismetSystemLibrary.IsValid` (`self.CurrentUser`))) (and _free_2 (`KismetSystemLibrary.IsValid` (`self.CurrentProcessingTarget`))))
            (set `self.CurrentUser` Player)
            (goto _label)))))))

(fn `OnProcessingFinished`
  (`/Game/Feastivus/Blueprints/BPFL_FeastivusAPI.DestroyActorAndAttachedActors` (`self.HoldingObject`))
  (set `self.HoldingObject` null)
  (set `/Game/Feastivus/Blueprints/Gameplay/BP_Player.ProcessingBench` null (`self.CurrentUser`))
  (`self.ResetCurrentUserAndChoppingTarget`
    (:`execute`
      (return))))

(fn `SpawnProcessingResult`
  (params (ObjectClass :type "/Game/Feastivus/Blueprints/Gameplay/BP_DynamicObject Class Reference"))
  (returns (SpawnedObject :type "/Game/Feastivus/Blueprints/Gameplay/BP_DynamicObject Object Reference"))
  (if (`KismetSystemLibrary.IsValidClass` ObjectClass)
    (bind _returnvalue (`|SpawnActorFromClass` ObjectClass (`KismetMathLibrary.MakeTransform` (0.0 0.0 0.0)) "AlwaysSpawn" "OverrideRootScale" null null))
    (return _returnvalue)))

(fn `UserConstructionScript`
  (`parent.UserConstructionScript`))