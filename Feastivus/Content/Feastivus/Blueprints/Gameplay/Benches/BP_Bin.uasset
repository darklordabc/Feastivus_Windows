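; BP_Bin is a kitchen bin bench that disposes of what a player brings to it, implemented entirely in InteractWith.
; Ingredient containers are emptied rather than destroyed, and other objects flagged CanBePutToBin are destroyed from the player's hands.
; Dishes without that flag are swapped for a freshly spawned BP_Plate and destroyed with their attached actors.
; Handled cases report success without starting processing, while an invalid object prints an error and fails.
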(fn `InteractWith`
  (params (Object :type "/Game/Feastivus/Blueprints/Gameplay/BP_DynamicObject Object Reference") (Player :type "/Game/Feastivus/Blueprints/Gameplay/BP_Player Object Reference"))
  (returns (bStartProcessing :type Boolean) (bSuccess :type Boolean))
  (`/Engine/EditorBlueprintResources/StandardMacros.IsValid` Object
    (:`Is Valid`
      (`/Game/Feastivus/Blueprints/BPML_FeastivusAPI.IsObjectChildOf` Object "/Game/Feastivus/Blueprints/Gameplay/Tools/BP_IngredientContainer.BP_IngredientContainer_C"
        (:`True`
          (bind _asbp_ingredient_container (cast `/Game/Feastivus/Blueprints/Gameplay/Tools/BP_IngredientContainer` Object)
            (:`then`
              (`/Game/Feastivus/Blueprints/Gameplay/Tools/BP_IngredientContainer.DestroyAllIngredients` _asbp_ingredient_container)
              (return false true))
            (:`CastFailed`
              (if (`/Game/Feastivus/Blueprints/Gameplay/BP_DynamicObject.bCanBePutToBin` Object) :!label _label
                (`self.DestroyHoldingObject` Player)
                (return false true)
                (else
                  _)))))
        (:`False`
          (goto _label)))
      (if (`KismetMathLibrary.ClassIsChildOf` (`GameplayStatics.GetObjectClass` Object) "/Game/Feastivus/Blueprints/Gameplay/Dishes/BP_Dish.BP_Dish_C")
        (bind _returnvalue (`|SpawnActorFromClass` "/Game/Feastivus/Blueprints/Gameplay/Tools/BP_Plate.BP_Plate_C" (`self.GetTransform` Object) "AlwaysSpawn" "OverrideRootScale" null null))
        (`/Game/Feastivus/Blueprints/BPFL_FeastivusAPI.ReplaceObject` Object _returnvalue)
        (`/Game/Feastivus/Blueprints/BPFL_FeastivusAPI.DestroyActorAndAttachedActors` Object)
        (return false true)))
    (:`Is Not Valid`
      (`KismetSystemLibrary.PrintString` "Bin target is nullptr!" true true (struct :`R` 1.0 :`G` 0.056108 :`A` 1.0) 10.0)
      (return false false))))

(fn `UserConstructionScript`
  (`parent.UserConstructionScript`))