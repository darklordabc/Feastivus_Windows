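; BP_ServingTable is a kitchen bench where players serve held dishes to fulfil orders.
; InteractWith accepts only BP_Dish objects and compares their class against the orders in the kitchen GameState.
; On the first match it swaps the player's dish for a spawned BP_DirtyPlate and multicasts removal of that order's widget.
; It never starts processing, and success reflects whether the plate was handed over.
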(fn `InteractWith`
  (params (Object :type "/Game/Feastivus/Blueprints/Gameplay/BP_DynamicObject Object Reference") (Player :type "/Game/Feastivus/Blueprints/Gameplay/BP_Player Object Reference"))
  (returns (bStartProcessing :type Boolean) (bSuccess :type Boolean))
  (`/Engine/EditorBlueprintResources/StandardMacros.IsValid` Object
    (:`Is Valid`
      (`/Game/Feastivus/Blueprints/BPML_FeastivusAPI.IsObjectChildOf` Object "/Game/Feastivus/Blueprints/Gameplay/Dishes/BP_Dish.BP_Dish_C"
        (:`True`
          (bind _asbp_game_state_kitchen_base (`/Game/Feastivus/Blueprints/BPML_FeastivusAPI.GetGameStateKitchen`)
            (:`then`
              (for (_array_element _array_index) (`/Game/Feastivus/Blueprints/BP_GameStateKitchenBase.Orders` _asbp_game_state_kitchen_base)
                (if (== (`.Dish_5_DEFB40AF4E47E803488B449D7D0B7282` (break `/Game/Feastivus/Recipes/S_Order` _array_element)) (`GameplayStatics.GetObjectClass` Object))
                  (bind _returnvalue (`|SpawnActorFromClass` "/Game/Feastivus/Blueprints/Gameplay/Tools/BP_DirtyPlate.BP_DirtyPlate_C" (`self.GetTransform` Object) "AlwaysSpawn" "OverrideRootScale" null null))
                  (`/Game/Feastivus/Blueprints/Gameplay/BP_Player.DestroyHoldingObject` Player)
                  (bind _success (`/Game/Feastivus/Blueprints/Gameplay/BP_Player.SetHoldingObject` Player _returnvalue))
                  (bind _asbp_game_state_kitchen_base_2 (`/Game/Feastivus/Blueprints/BPML_FeastivusAPI.GetGameStateKitchen`)
                    (:`then`
                      (`/Game/Feastivus/Blueprints/BP_GameStateKitchenBase.MulticastRemoveOrderWidget` _asbp_game_state_kitchen_base_2 _array_index))
                    (:`CastFailed`
                      _))
                  (return false _success)))
              (return false false))))
        (:`False`
          _)))
    (:`Is Not Valid`
      (`KismetSystemLibrary.PrintString` "Serving target is nullptr!" true true (struct :`R` 1.0 :`G` 0.056108 :`A` 1.0) 10.0)))
  (return false false))

(fn `UserConstructionScript`
  (`parent.UserConstructionScript`))