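; BP_PlateTable is a bench in Feastivus that restricts the objects it takes to clean plate stacks and plates.
; Its InteractWith override forwards those classes, or an interaction with no valid object, to the parent bench logic and returns its result.
; Any other valid object is refused, returning false for both StartProcessing and Success.
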(fn `InteractWith`
  (params (Object :type "/Game/Feastivus/Blueprints/Gameplay/BP_DynamicObject Object Reference") (Player :type "/Game/Feastivus/Blueprints/Gameplay/BP_Player Object Reference"))
  (returns (bStartProcessing :type Boolean) (bSuccess :type Boolean))
  (bind _returnvalue (`GameplayStatics.GetObjectClass` Object))
  (if (not (or (`KismetMathLibrary.ClassIsChildOf` _returnvalue "/Game/Feastivus/Blueprints/Gameplay/Tools/BP_CleanPlateStack.BP_CleanPlateStack_C") (`KismetMathLibrary.ClassIsChildOf` _returnvalue "/Game/Feastivus/Blueprints/Gameplay/Tools/BP_Plate.BP_Plate_C")))
    (`/Engine/EditorBlueprintResources/StandardMacros.IsValid` (`local.Object`)
      (:`Is Valid`
        (return false false))
      (:`Is Not Valid`
        _)))
  (bind (_bstartprocessing _bsuccess) (`parent.InteractWith` Object Player))
  (return _bstartprocessing _bsuccess))

(fn `UserConstructionScript`
  (`parent.UserConstructionScript`))