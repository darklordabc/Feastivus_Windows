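; BP_Plate is a kitchen plate that collects ingredients and turns into a finished dish.
; TakeIngredient checks the current contents plus the new ingredient against DT_Recipes, then attaches accepted ingredients to its trigger box at a random yaw.
; When the matched recipe has a valid Dish class, it spawns that dish, swaps it in for the plate and destroys the plate with its attachments.
; Stack events hide the layout widget while stacked and show it once removed.
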(event `/Game/Feastivus/Blueprints/Gameplay/Tools/BPI_Stackable.OnStacked`
  (params (Stack :type "/Game/Feastivus/Blueprints/Gameplay/Tools/BP_Stack Object Reference"))
  (`self.Event Set Layout Widget Visibility` true))

(event `/Game/Feastivus/Blueprints/Gameplay/Tools/BPI_Stackable.OnRemovedFromStack`
  (params (Stack :type "/Game/Feastivus/Blueprints/Gameplay/Tools/BP_Stack Object Reference"))
  (`self.Event Set Layout Widget Visibility` false))

(event `Event Set Layout Widget Visibility`
  (params (Hidden :type Boolean))
  (`SceneComponent.SetHiddenInGame` (`self.Widget`) Hidden false))

(fn `TakeIngredient`
  (params (Ingredient :type "/Game/Feastivus/Blueprints/Gameplay/Ingredients/BP_Ingredient Object Reference"))
  (returns (Success :type Boolean))
  (bind _ingredientclasses (`/Game/Feastivus/Blueprints/BPFL_FeastivusAPI.GetIngredientClasses` (`self.Ingredients`)))
  (bind (_success _recipe) (`IngredientChecker.CheckIngredient` (`GameplayStatics.GetObjectClass` Ingredient) _ingredientclasses "/Game/Feastivus/Recipes/DT_Recipes.DT_Recipes"))
  (if _success
    (bind _success_2 (`parent.TakeIngredient` Ingredient))
    (if _success_2
      (`/Game/Feastivus/Blueprints/BPFL_FeastivusAPI.FreeObjectHolder` Ingredient)
      (bind _attachedobject (`/Game/Feastivus/Blueprints/BPFL_FeastivusAPI.AttachObject` Ingredient (`self.TriggerBox`)))
      (`self.K2_SetActorRelativeRotation` _attachedobject (`KismetMathLibrary.MakeRotator` 0.0 0.0 (`KismetMathLibrary.RandomFloatInRange` 0.0 360.0)) false false)
      (bind (_name _ingredients _dish) (break `Recipe` _recipe))
      (if (`KismetSystemLibrary.IsValidClass` _dish)
        ;[0.5492 1 0.6971] Dish is ready
        (bind _returnvalue (`|SpawnActorFromClass` _dish (`self.GetTransform` self) "AlwaysSpawn" "OverrideRootScale" null null))
        (bind _asbp_dynamic_object (cast `/Game/Feastivus/Blueprints/Gameplay/BP_DynamicObject` _returnvalue)
          (:`then`
            (`/Game/Feastivus/Blueprints/BPFL_FeastivusAPI.ReplaceObject` self _asbp_dynamic_object)
            (`/Game/Feastivus/Blueprints/BPFL_FeastivusAPI.DestroyActorAndAttachedActors` self))
          (:`CastFailed`
            (return false))))
      (return true)
      (else
        (return false)))
    (else
      (return false))))

(fn `UserConstructionScript`
  (`parent.UserConstructionScript`))