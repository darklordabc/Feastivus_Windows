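; BP_Pan is a cooking container that fries the ingredients placed in it.
; GetRecipes returns every row of the DT_PanRecipes data table as the pan's recipes.
; FinishCooking asks each ingredient for its frying target class, destroys the ingredients, then spawns those classes attached to the TriggerBox as the new contents.
; It then multicasts the cooking result, passing the last class from the spawn loop.
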(fn `FinishCooking`
  (returns (bSuccess :type Boolean))
  (locals (IngredientsToSpawn :type "Array of /Game/Feastivus/Blueprints/Gameplay/Ingredients/BP_Ingredient Class Reference"))
  (for _array_element (`self.Ingredients`)
    (bind _target (message `/Game/Feastivus/Blueprints/Gameplay/Ingredients/BPI_Friable.GetFryingTarget` _array_element))
    (`KismetArrayLibrary.Array_Add` (`local.IngredientsToSpawn`) _target))
  (`self.DestroyAllIngredients`)
  (for _array_element_2 (`local.IngredientsToSpawn`)
    (bind _returnvalue (`|SpawnActorFromClass` _array_element_2 (`self.GetTransform`) "Undefined" "OverrideRootScale" null null))
    (`/Game/Feastivus/Blueprints/BPFL_FeastivusAPI.AttachObject` _returnvalue (`self.TriggerBox`))
    (`KismetArrayLibrary.Array_Add` (`self.Ingredients`) _returnvalue))
  (`self.MulticastSetCookingResult` _array_element_2)
  (return true))

(fn `GetRecipes`
  (returns (Recipes :type "Array of Recipe Structure"))
  (locals (RecipesLocal :type "Array of Recipe Structure"))
  (bind _outrownames (`DataTableFunctionLibrary.GetDataTableRowNames` "/Game/Feastivus/Blueprints/Gameplay/Tools/CookingContainers/DT_PanRecipes.DT_PanRecipes"))
  (for _array_element _outrownames
    (bind _returnvalue (`|GetDataTableRow` "/Game/Feastivus/Blueprints/Gameplay/Tools/CookingContainers/DT_PanRecipes.DT_PanRecipes" _array_element)
      (:`then`
        (`KismetArrayLibrary.Array_Add` (`local.RecipesLocal`) _returnvalue))))
  (return (`local.RecipesLocal`)))

(fn `UserConstructionScript`
  (`parent.UserConstructionScript`))