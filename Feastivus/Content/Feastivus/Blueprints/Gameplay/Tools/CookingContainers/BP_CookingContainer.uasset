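; Cooking container that takes recipe-valid ingredients and cooks them while attached to a lava bench, with GetRecipes left empty here.
; Added ingredients are hidden inside and roll back cooking progress.
; The server advances cooking, then overtime, finishing completed recipes once or destroying the contents when overtime expires.
; Plates collect finished contents, while the layout widget shows progress and overtime danger, with multicasts updating icons and resets.
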(event `self.ReceiveBeginPlay`
  (`parent.ReceiveBeginPlay`))

(event `self.ReceiveTick`
  (params (DeltaSeconds :type "Float (single-precision)"))
  (`parent.ReceiveTick` DeltaSeconds)
  (`|ExecutionSequence`
    (:`then_0`
      (`/Engine/EditorBlueprintResources/StandardMacros.IsValid` (`self.GetLayoutWidget`)
        (:`Is Valid`
          (`self.SwitchIsOnLavaBench`
            (:`then`
              (set `/Game/Feastivus/Blueprints/Widgets/BPW_IconLayout2x2.ProgressPercent` (`self.CookingPercent`) (`self.GetLayoutWidget`))
              (`/Game/Feastivus/Blueprints/Widgets/BPW_IconLayout2x2.ToggleProgressDanger` (`self.GetLayoutWidget`) (> (`self.OvertimePercent`) 0.0)))
            (:`CastFailed`
              (`/Game/Feastivus/Blueprints/Widgets/BPW_IconLayout2x2.ToggleProgressDanger` (`self.GetLayoutWidget`) false))))))
    (:`then_1`
      (`/Engine/EditorBlueprintResources/ActorMacros.Switch Has Authority`
        (:`Authority`
          (`self.SwitchIsOnLavaBench`
            (:`then`
              (if (`self.HasAtLeastOneIngredient`)
                (bind _returnvalue (`self.IncrementPercentTimer` (`self.CookingTime`) (`self.CookingPercent`)))
                (if (>= _returnvalue 1.0)
                  (bind _returnvalue_2 (`self.IncrementPercentTimer` (`self.Overtime`) (`self.OvertimePercent`)))
                  (if (>= _returnvalue_2 1.0)
                    (`self.Reset` false)
                    (elif (`self.bRecipeComplete`)
                      (`/Engine/EditorBlueprintResources/StandardMacros.DoOnce` false :!label _label
                        (:`Completed`
                          (`self.FinishCooking`))))))))))))))

(event `ResetDoOnces`
  (goto _label :!via `Reset`))

(event `MulticastSetCookingResult`
  (params (IngredientClass :type "/Game/Feastivus/Blueprints/Gameplay/Ingredients/BP_Ingredient Class Reference"))
  (bind _asbpw_icon_layout_2x_2 (`self.GetLayoutWidget`))
  (bind _texture (`/Game/Feastivus/Blueprints/BPFL_FeastivusAPI.GetIconTexture` IngredientClass))
  (`/Game/Feastivus/Blueprints/Widgets/BPW_IconLayout2x2.SetEnabledSlots` _asbpw_icon_layout_2x_2 1)
  (`/Game/Feastivus/Blueprints/Widgets/BPW_IconLayout2x2.SetSlotIconTexture` _asbpw_icon_layout_2x_2 _texture 0))

(event `MulticastHideProgressBar`
  (set `/Game/Feastivus/Blueprints/Widgets/BPW_IconLayout2x2.ProgressPercent` 0.0 (`self.GetLayoutWidget`)))

(fn `FinishCooking`
  (returns (bSuccess :type Boolean))
  (`self.DestroyAllIngredients`)
  (return true))

(fn `GetRecipes`
  (returns (Recipes :type "Array of Recipe Structure"))
  (return))

(fn `IncrementPercentTimer`
  (params (Duration :type "Float (double-precision)") (CurrentValue :type "Float (double-precision) (by ref)"))
  (returns (ReturnValue :type "Float (double-precision)"))
  (bind _returnvalue (`KismetMathLibrary.FMin` (+ (* (`GameplayStatics.GetWorldDeltaSeconds`) (/ 1.0 Duration)) CurrentValue) 1.0))
  (`|VariableSetRef` CurrentValue _returnvalue)
  (return _returnvalue))

(fn `InteractWith`
  (params (Object :type "/Game/Feastivus/Blueprints/Gameplay/BP_DynamicObject Object Reference") (Player :type "/Game/Feastivus/Blueprints/Gameplay/BP_Player Object Reference"))
  (returns (bStartProcessing :type Boolean) (bSuccess :type Boolean))
  (bind _asbp_plate (cast `/Game/Feastivus/Blueprints/Gameplay/Tools/BP_Plate` Object)
    (:`then`
      (if (`self.IsCookingFinished`)
        (for _array_element (`self.Ingredients`)
          (`self.InteractWith` _asbp_plate _array_element (`local.Player`)))
        (`self.Reset` true)
        (return false true)))
    (:`CastFailed`
      (bind (_bstartprocessing _bsuccess) (`parent.InteractWith` Object Player))
      (return _bstartprocessing _bsuccess))))

(fn `IsCookingFinished`
  (returns (bFinished :type Boolean))
  (return (and (`self.bRecipeComplete`) (== (`self.CookingPercent`) 1.0))))

(fn `Reset`
  (params (bDontDestroyActors :type Boolean))
  (if bDontDestroyActors
    (`KismetArrayLibrary.Array_Clear` (`self.Ingredients`))
    (else
      (`self.DestroyAllIngredients`)))
  (`self.MulticastResetLayoutWidget`)
  (set `self.CookingPercent` 0.0)
  (set `self.OvertimePercent` 0.0)
  (`self.ResetDoOnces`)
  (`self.MulticastHideProgressBar`)
  (return))

(fn `TakeIngredient`
  (params (Ingredient :type "/Game/Feastivus/Blueprints/Gameplay/Ingredients/BP_Ingredient Object Reference"))
  (returns (Success :type Boolean))
  (bind _ingredient (`local.Ingredient`))
  (if (== (`KismetArrayLibrary.Array_Length` (`self.Ingredients`)) (`self.Slots`))
    (return false)
    (else
      (bind _recipes (`self.GetRecipes`))
      (bind _ingredientclasses (`/Game/Feastivus/Blueprints/BPFL_FeastivusAPI.GetIngredientClasses` (`self.Ingredients`)))
      (bind (_bsuccess _dishindex) (`IngredientChecker.CheckIngredient` (`GameplayStatics.GetObjectClass` (`local.Ingredient`)) _ingredientclasses _recipes))
      (if _bsuccess
        (bind _success (`parent.TakeIngredient` (`local.Ingredient`)))
        (if _success
          (`/Game/Feastivus/Blueprints/BPFL_FeastivusAPI.FreeObjectHolder` _ingredient)
          (bind _attachedobject (`/Game/Feastivus/Blueprints/BPFL_FeastivusAPI.AttachObject` _ingredient (`self.TriggerBox`) "None" "SnapToTarget"))
          (`self.SetActorHiddenInGame` _attachedobject true)
          (set `self.CookingPercent` (`KismetMathLibrary.FMax` 1e-05 (- (`self.CookingPercent`) (/ 1.0 (`KismetMathLibrary.Conv_IntToDouble` (`self.Slots`))))))
          (set `self.OvertimePercent` 0.0)
          (if (`KismetArrayLibrary.Array_IsValidIndex` _recipes _dishindex)
            (set `self.bRecipeComplete` true))
          (return true)
          (else
            (return false)))
        (else
          (return false))))))

(fn `UserConstructionScript`
  (`parent.UserConstructionScript`))