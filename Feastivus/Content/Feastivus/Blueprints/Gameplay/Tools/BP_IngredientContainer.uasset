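; BP_IngredientContainer is a gameplay tool that collects ingredients up to its slot count and displays their icons.
; InteractWith passes ingredient objects to TakeIngredient, which rejects duplicates or overflow and never starts processing.
; Each accepted ingredient sets its slot icon on a 2x2 layout widget, whose enabled slots are set on BeginPlay.
; DestroyAllIngredients destroys the stored actors, empties the array and resets the widget through a multicast event.
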(event `self.ReceiveBeginPlay`
  (`parent.ReceiveBeginPlay`)
  (`/Game/Feastivus/Blueprints/Widgets/BPW_IconLayout2x2.SetEnabledSlots` (`self.GetLayoutWidget`) (`self.Slots`)))

(event `Event Set Layout Widget Icon`
  (params (IconTexture :type "Texture2D Object Reference") (Slot :type Integer))
  (`/Game/Feastivus/Blueprints/Widgets/BPW_IconLayout2x2.SetSlotIconTexture` (`self.GetLayoutWidget`) IconTexture Slot))

(event `MulticastResetLayoutWidget`
  (bind _asbpw_icon_layout_2x_2 (`self.GetLayoutWidget`))
  (`/Game/Feastivus/Blueprints/Widgets/BPW_IconLayout2x2.ClearAllSlots` _asbpw_icon_layout_2x_2)
  (`/Game/Feastivus/Blueprints/Widgets/BPW_IconLayout2x2.SetEnabledSlots` _asbpw_icon_layout_2x_2 (`self.Slots`)))

(fn `DestroyAllIngredients`
  (`/Game/Feastivus/Blueprints/BPFL_FeastivusAPI.DestroyArrayOfActors` (`self.Ingredients`))
  (`KismetArrayLibrary.Array_Clear` (`self.Ingredients`))
  (`self.MulticastResetLayoutWidget`))

(fn `GetAllIngredients`
  (returns (Ingredients :type "Array of /Game/Feastivus/Blueprints/Gameplay/Ingredients/BP_Ingredient Object Reference"))
  (return (`self.Ingredients`)))

(fn `GetLayoutWidget`
  (returns (`AsBPW Icon Layout 2x 2` :type "/Game/Feastivus/Blueprints/Widgets/BPW_IconLayout2x2 Object Reference"))
  (return (cast `/Game/Feastivus/Blueprints/Widgets/BPW_IconLayout2x2` (`WidgetComponent.GetUserWidgetObject` (`self.WidgetIconLayout`)) :!pure true)))

(fn `HasAtLeastOneIngredient`
  (returns (bSuccess :type Boolean))
  (return (> (`KismetArrayLibrary.Array_Length` (`self.Ingredients`)) 0)))

(fn `InteractWith`
  (params (Object :type "/Game/Feastivus/Blueprints/Gameplay/BP_DynamicObject Object Reference") (Player :type "/Game/Feastivus/Blueprints/Gameplay/BP_Player Object Reference"))
  (returns (bStartProcessing :type Boolean) (bSuccess :type Boolean))
  (bind _asbp_ingredient (cast `/Game/Feastivus/Blueprints/Gameplay/Ingredients/BP_Ingredient` Object)
    (:`then`
      (bind _success (`self.TakeIngredient` _asbp_ingredient))
      (return false _success))
    (:`CastFailed`
      (return false false))))

(fn `TakeIngredient`
  (params (Ingredient :type "/Game/Feastivus/Blueprints/Gameplay/Ingredients/BP_Ingredient Object Reference"))
  (returns (Success :type Boolean))
  (locals (IsSuccess :type Boolean))
  (bind _output_get (set `local.IsSuccess` (and (> (`self.Slots`) (`KismetArrayLibrary.Array_Length` (`self.Ingredients`))) (not (`KismetArrayLibrary.Array_Contains` (`self.Ingredients`) Ingredient)))))
  (if _output_get
    (bind _returnvalue (`KismetArrayLibrary.Array_AddUnique` (`self.Ingredients`) Ingredient))
    (`self.Event Set Layout Widget Icon` (`.IconTexture_4_8E1524674FDD5ABEE7D6ECABD6ADFE62` (break `/Game/Feastivus/Blueprints/Gameplay/S_ObjectUIInfo` (`/Game/Feastivus/Blueprints/Gameplay/Ingredients/BP_Ingredient.UIInfo` Ingredient))) _returnvalue))
  (return (`local.IsSuccess`)))

(fn `UserConstructionScript`
  (`parent.UserConstructionScript`))