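; BP_FixedStack is a stack tool in Feastivus that only accepts objects of one configured class, filtering additions before passing them to its parent.
; It can spawn and pack new items of that class, or remove and destroy the last one.
; With MergeOnInteract on, interacting with a matching item or same-class fixed stack spawns equivalent items here, then frees and destroys the incoming actor with its attachments.
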(event `self.AddObject`
  (params (Object :type "/Game/Feastivus/Blueprints/Gameplay/BP_DynamicObject Object Reference"))
  (if (`KismetMathLibrary.ClassIsChildOf` (`GameplayStatics.GetObjectClass` Object) (`self.ObjectClass`))
    (`parent.AddObject` Object)))

(fn `InteractWith`
  (params (Object :type "/Game/Feastivus/Blueprints/Gameplay/BP_DynamicObject Object Reference") (Player :type "/Game/Feastivus/Blueprints/Gameplay/BP_Player Object Reference"))
  (returns (bStartProcessing :type Boolean) (bSuccess :type Boolean))
  (bind _object (`local.Object`))
  (if (`self.bMergeOnInteract`)
    (`/Game/Feastivus/Blueprints/BPML_FeastivusAPI.IsObjectChildOf` (`local.Object`) (`self.ObjectClass`)
      (:`True`
        (`self.SpawnAndAddObject`)
        (`/Game/Feastivus/Blueprints/BPFL_FeastivusAPI.FreeObjectHolder` _object :!label _label)
        (`/Game/Feastivus/Blueprints/BPFL_FeastivusAPI.DestroyActorAndAttachedActors` _object)
        (return false true))
      (:`False`
        (bind _asbp_fixed_stack (cast `/Game/Feastivus/Blueprints/Gameplay/Tools/BP_FixedStack` (`local.Object`))
          (:`then`
            (if (== (`self.ObjectClass`) (`/Game/Feastivus/Blueprints/Gameplay/Tools/BP_FixedStack.ObjectClass` _asbp_fixed_stack))
              (for _ (`/Game/Feastivus/Blueprints/Gameplay/Tools/BP_Stack.Objects` _asbp_fixed_stack)
                (`self.SpawnAndAddObject`))
              (goto _label)))
          (:`CastFailed`
            (bind (_bstartprocessing _bsuccess) (`parent.InteractWith` Object Player :!label _label_2))
            (return _bstartprocessing _bsuccess)))))
    (else
      (goto _label_2))))

(fn `RemoveLast`
  (bind _objects (`self.Objects`))
  (if (> (`KismetArrayLibrary.Array_Length` _objects) 0)
    (bind _detachedobject (`self.RemoveObject` (`KismetArrayLibrary.Array_LastIndex` _objects) true))
    (`self.K2_DestroyActor` _detachedobject)))

(fn `SpawnAndAddObject`
  (bind _returnvalue (`|SpawnActorFromClass` (`self.ObjectClass`) (`KismetMathLibrary.MakeTransform` (0.0 0.0 0.0)) "Undefined" "OverrideRootScale" null null))
  (`self.AddObject` _returnvalue)
  (`self.PackObjects`))

(fn `UserConstructionScript`
  (`parent.UserConstructionScript`))