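; BP_Stack is a gameplay tool that holds a vertical pile of objects that players take from one at a time.
; Objects attach to its TriggerBox at index-based height offsets, packed on construction and BeginPlay, and are notified when stacked or removed.
; Interaction hands the last object to a free player if pickup is available.
; When removal leaves one object, the stack replaces itself with it and destroys itself, unless told otherwise.
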(event `self.ReceiveBeginPlay`
  (`parent.ReceiveBeginPlay`)
  (`self.PackObjects`))

(fn `AddObject`
  (params (Object :type "/Game/Feastivus/Blueprints/Gameplay/BP_DynamicObject Object Reference"))
  (bind _returnvalue (`KismetArrayLibrary.Array_AddUnique` (`self.Objects`) Object))
  (if (`KismetArrayLibrary.Array_IsValidIndex` (`self.Objects`) _returnvalue)
    (bind _attachedobject (`/Game/Feastivus/Blueprints/BPFL_FeastivusAPI.AttachObject` Object (`self.TriggerBox`) "None" "SnapToTarget"))
    (`self.K2_SetActorRelativeLocation` _attachedobject (`KismetMathLibrary.MakeVector` 0.0 0.0 (* _returnvalue (`self.VerticalOffset`))) false true)
    (message `/Game/Feastivus/Blueprints/Gameplay/Tools/BPI_Stackable.OnStacked` _attachedobject self)
    (return)
    (else
      (return))))

(fn `InteractWith`
  (params (Object :type "/Game/Feastivus/Blueprints/Gameplay/BP_DynamicObject Object Reference") (Player :type "/Game/Feastivus/Blueprints/Gameplay/BP_Player Object Reference"))
  (returns (bStartProcessing :type Boolean) (bSuccess :type Boolean))
  (bind _free (`/Game/Feastivus/Blueprints/Gameplay/BP_Player.IsFree` Player))
  (if (and (`self.bAvailableToPickup`) _free)
    (bind _detachedobject (`self.RemoveObject` (`KismetArrayLibrary.Array_LastIndex` (`self.Objects`))))
    (bind _success (`/Game/Feastivus/Blueprints/Gameplay/BP_Player.SetHoldingObject` Player _detachedobject))
    (return false _success)
    (else
      (return false false))))

(fn `PackObjects`
  (for (_array_element _array_index) (`self.Objects`)
    (bind _attachedobject (`/Game/Feastivus/Blueprints/BPFL_FeastivusAPI.AttachObject` _array_element (`self.TriggerBox`) "None" "SnapToTarget"))
    (`self.K2_SetActorRelativeLocation` _attachedobject (`KismetMathLibrary.MakeVector` 0.0 0.0 (* _array_index (`self.VerticalOffset`))) false true)
    (message `/Game/Feastivus/Blueprints/Gameplay/Tools/BPI_Stackable.OnStacked` _attachedobject self)))

(fn `RemoveObject`
  (params (Index :type Integer) (bDontDestroyStack :type Boolean))
  (returns (DetachedObject :type "/Game/Feastivus/Blueprints/Gameplay/BP_DynamicObject Object Reference"))
  (bind _detachedobject (`/Game/Feastivus/Blueprints/BPFL_FeastivusAPI.DetachObject` (`|GetArrayItem` (`self.Objects`) Index)))
  (message `/Game/Feastivus/Blueprints/Gameplay/Tools/BPI_Stackable.OnRemovedFromStack` _detachedobject self)
  (`KismetArrayLibrary.Array_Remove` (`self.Objects`) Index)
  (if (and (== (`KismetArrayLibrary.Array_Length` (`self.Objects`)) 1) (not bDontDestroyStack))
    (bind _detachedobject_2 (`self.RemoveObject` 0))
    (`/Game/Feastivus/Blueprints/BPFL_FeastivusAPI.ReplaceObject` self _detachedobject_2)
    (`self.K2_DestroyActor`))
  (return _detachedobject))

(fn `UserConstructionScript`
  (`parent.UserConstructionScript`)
  (`self.PackObjects`))