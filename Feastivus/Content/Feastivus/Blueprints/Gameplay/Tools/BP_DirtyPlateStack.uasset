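; BP_DirtyPlateStack is a stack tool that holds dirty plates in the Feastivus gameplay.
; AddDirtyPlate spawns a BP_DirtyPlate, adds it to the inherited object list and repacks the stack.
; RemoveDirtyPlate pops the last object, if any, and destroys it.
; GetWashingTarget returns BP_Stack as the washing target, and the event graph holds only disabled default events.
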(fn `AddDirtyPlate`
  (bind _returnvalue (`|SpawnActorFromClass` "/Game/Feastivus/Blueprints/Gameplay/Tools/BP_DirtyPlate.BP_DirtyPlate_C" (`KismetMathLibrary.MakeTransform` (0.0 0.0 0.0)) "Undefined" "OverrideRootScale" null null))
  (`self.AddObject` _returnvalue)
  (`self.PackObjects`))

(fn `GetWashingTarget`
  (returns (WashingTarget :type "/Game/Feastivus/Blueprints/Gameplay/BP_DynamicObject Class Reference"))
  (return "/Game/Feastivus/Blueprints/Gameplay/Tools/BP_Stack.BP_Stack_C"))

(fn `RemoveDirtyPlate`
  (bind _objects (`self.Objects`))
  (if (> (`KismetArrayLibrary.Array_Length` _objects) 0)
    (bind _detachedobject (`self.RemoveObject` (`KismetArrayLibrary.Array_LastIndex` _objects)))
    (`self.K2_DestroyActor` _detachedobject)))

(fn `UserConstructionScript`
  (`parent.UserConstructionScript`))