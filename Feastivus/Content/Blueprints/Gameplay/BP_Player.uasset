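; Networked player character that walks, picks up and drops objects, and interacts with stations under a shared BP_Camera view set on clients.
; Movement turns toward input before moving and is blocked while a ProcessingBench is set; pressing Interact then interrupts processing.
; TriggerBox overlaps filtered by class and interface choose targets for server interaction events and authority-side outlining.
; HoldingObject's OnRep attaches the carried object, or detaches and ground-snaps it, on authority.
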(event `self.ReceiveTick`
  (params (DeltaSeconds :type "Float (single-precision)"))
  (`/Engine/EditorBlueprintResources/ActorMacros.Switch Has Authority`
    (:`Authority`
      (`self.Event Check Interact Target`))))

(event `Event Check Interact Target`
  (bind _interactoutlinetarget (`self.InteractOutlineTarget`))
  ;[1 0.7643 0.2543] Outline interact target
  (bind _object (`self.CheckInteractTarget` "/Game/Blueprints/Gameplay/BP_GameplayObject.BP_GameplayObject_C" null true)
    (:`Success`
      (if (and (!= (`self.InteractOutlineTarget`) _object) (`KismetSystemLibrary.IsValid` (`self.InteractOutlineTarget`)))
        (`/Game/Blueprints/BPFL_FeastivusAPI.FeastivusOutlineActor` false (`self.InteractOutlineTarget`)))
      (bind _output_get (set `self.InteractOutlineTarget` _object))
      (`/Game/Blueprints/BPFL_FeastivusAPI.FeastivusOutlineActor` true _output_get))
    (:`Failure`
      (`/Engine/EditorBlueprintResources/StandardMacros.IsValid` _interactoutlinetarget
        (:`Is Valid`
          (`/Game/Blueprints/BPFL_FeastivusAPI.FeastivusOutlineActor` false _interactoutlinetarget)
          (set `self.InteractOutlineTarget` null))))))

(event `Event Any Key Pressed`
  ;[0.6878 1 0.8662] Any key pressed (unused)
  (`/Engine/EditorBlueprintResources/StandardMacros.IsValid` (`self.ProcessingBench`)
    (:`Is Valid`
      (message `/Game/Blueprints/Gameplay/Benches/BPI_IngredientProcessor.InterruptProcessing` (`self.ProcessingBench`)))))

(event `Key|AnyKey` :consume false
  (params (Key :type "Key Structure"))
  ;[0.6878 1 0.8662] Any key pressed (unused)
)

(event `self.ReceiveBeginPlay`
  ;[0.02011 0.2862 1] Init camera
  (`/Engine/EditorBlueprintResources/ActorMacros.Switch Has Authority`
    (:`Remote`
      (bind _outactors (`GameplayStatics.GetAllActorsOfClass` "/Game/Blueprints/Gameplay/BP_Camera.BP_Camera_C"))
      (`PlayerController.SetViewTargetWithBlend` (`GameplayStatics.GetPlayerController` 0) (`|GetArrayItem` _outactors) 0.0 "VTBlend_Linear" 0.0 false))))

(event `InputAxis|VerticalWalk`
  (params (AxisValue :type "Float (single-precision)"))
  (bind _returnvalue (`self.GetController`))
  ;[0.5345 1 0.6157] Movement
  (`/Engine/EditorBlueprintResources/StandardMacros.IsValid` (`self.ProcessingBench`) :!label _label
    (:`Is Not Valid`
      (bind _returnvalue_2 (`KismetMathLibrary.MakeVector` AxisValue (stale `InputAxis|HorizontalWalk` AxisValue)))
      (if (> (`KismetMathLibrary.VSize` _returnvalue_2) 0.25)
        (bind _returnvalue_3 (`KismetMathLibrary.Conv_VectorToRotator` _returnvalue_2))
        (`Controller.SetControlRotation` _returnvalue (`KismetMathLibrary.RInterpTo` (`Controller.GetControlRotation` _returnvalue) _returnvalue_3 (`GameplayStatics.GetWorldDeltaSeconds`) (`self.RotationSpeed`)))
        (if (<= (`KismetMathLibrary.VSize` (- (`KismetMathLibrary.Conv_RotatorToVector` (`Controller.GetControlRotation` (`self.GetController`))) _returnvalue_2)) (`self.MovementThreshold`))
          (`self.AddMovementInput` (`KismetMathLibrary.GetForwardVector` _returnvalue_3)))))))

(event `InputAxis|HorizontalWalk`
  (params (AxisValue :type "Float (single-precision)"))
  ;[0.5345 1 0.6157] Movement
  (goto _label))

(event `Event Server Drop`
  ;[1 0.5237 0.4034] Interact
  (bind _object (`self.CheckInteractTarget` "/Game/Blueprints/Gameplay/BP_StaticObject.BP_StaticObject_C" "/Game/Blueprints/Gameplay/BPI_Interactable.BPI_Interactable_C")
    (:`Success`
      (message `/Game/Blueprints/Gameplay/BPI_Interactable.InteractWith` _object (`self.HoldingObject`) self))
    (:`Failure`
      (set `self.HoldingObject` null))))

(event `InputAction|Interact`
  (params (Key :type "Key Structure"))
  ;[1 0.4253 0.8423] Interact Key Pressed
  (:`Pressed`
    (`/Engine/EditorBlueprintResources/StandardMacros.IsValid` (`self.ProcessingBench`)
      (:`Is Valid`
        (`self.Event Server Interrupt Processing`))
      (:`Is Not Valid`
        (`/Engine/EditorBlueprintResources/StandardMacros.IsValid` (`self.HoldingObject`)
          (:`Is Valid`
            (`self.Event Server Drop`))
          (:`Is Not Valid`
            (`self.Event Server Interact`)))))))

(event `Event Server Interact`
  ;[0.4951 0.8166 1] Interact (free hands)
  (bind _object (`self.CheckInteractTarget` "/Game/Blueprints/Gameplay/BP_StaticObject.BP_StaticObject_C" "/Game/Blueprints/Gameplay/BPI_Interactable.BPI_Interactable_C")
    (:`Success`
      (if (`KismetSystemLibrary.DoesImplementInterface` _object "/Game/Blueprints/Gameplay/BPI_Interactable.BPI_Interactable_C")
        (bind _startprocessing (message `/Game/Blueprints/Gameplay/BPI_Interactable.InteractWith` _object (`self.HoldingObject`) self))
        (if _startprocessing
          _)))
    (:`Failure`
      (bind _object_2 (`self.CheckInteractTarget` "/Game/Blueprints/Gameplay/BP_DynamicObject.BP_DynamicObject_C" "/Game/Blueprints/Gameplay/BPI_Pickable.BPI_Pickable_C")
        (:`Success`
          (bind _asbp_dynamic_object (cast `/Game/Blueprints/Gameplay/BP_DynamicObject` _object_2))
          (set `self.HoldingObject` _asbp_dynamic_object))))))

(event `Event Server Interrupt Processing`
  ;[1 0.4253 0.8423] Interact Key Pressed
  (`/Engine/EditorBlueprintResources/StandardMacros.IsValid` (`self.ProcessingBench`)
    (:`Is Valid`
      (message `/Game/Blueprints/Gameplay/Benches/BPI_IngredientProcessor.InterruptProcessing` (`self.ProcessingBench`)))))

(fn `IsFree`
  (returns (Free :type Boolean))
  (return (not (`KismetSystemLibrary.IsValid` (`self.HoldingObject`)))))

(fn `OnRep_HoldingObject`
  (bind _returnvalue (`SceneComponent.GetChildComponent` (`self.TriggerBox`) 0))
  (if (`KismetSystemLibrary.IsValid` (`self.HoldingObject`))
    (`/Engine/EditorBlueprintResources/ActorMacros.Switch Has Authority`
      (:`Authority`
        (`/Game/Blueprints/BPFL_FeastivusAPI.FeastivusAttach` (`self.HoldingObject`) (`self.TriggerBox`))))
    (else
      (`/Engine/EditorBlueprintResources/ActorMacros.Switch Has Authority`
        (:`Authority`
          (if (`KismetSystemLibrary.IsValid` _returnvalue)
            (bind _asbp_dynamic_object (cast `/Game/Blueprints/Gameplay/BP_DynamicObject` (`ActorComponent.GetOwner` _returnvalue)))
            (bind _detachedobject (`/Game/Blueprints/BPFL_FeastivusAPI.FeastivusDetach` _asbp_dynamic_object))
            (`/Game/Blueprints/Gameplay/BP_GameplayObject.SnapToGround` _detachedobject)))))))

(fn `UserConstructionScript`)