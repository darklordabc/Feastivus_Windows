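; BP_Bin is a bench Blueprint that acts as a bin for objects a player interacts with it using.
; Its InteractWith function empties ingredient containers by destroying their ingredients, leaving the container itself intact.
; Other objects flagged CanBePutToBin are passed to the player's SetHoldingObject and then destroyed.
; Both disposal paths return false, and the event graph holds only disabled default events.
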(fn `InteractWith`
  (params (Object :type "/Game/Blueprints/Gameplay/BP_DynamicObject Object Reference") (Player :type "/Game/Blueprints/Gameplay/BP_Player Object Reference"))
  (returns (StartProcessing :type Boolean))
  (`/Game/Blueprints/BPML_FeastivusAPI.IsObjectChildOf` Object "/Game/Blueprints/Gameplay/Tools/BP_IngredientContainer.BP_IngredientContainer_C"
    (:`True`
      (bind _asbp_ingredient_container (cast `/Game/Blueprints/Gameplay/Tools/BP_IngredientContainer` Object)
        (:`then`
          (`/Game/Blueprints/Gameplay/Tools/BP_IngredientContainer.DestroyAllIngredients` _asbp_ingredient_container)
          (return false))
        (:`CastFailed`
          (if (`/Game/Blueprints/Gameplay/BP_DynamicObject.bCanBePutToBin` Object) :!label _label
            (`/Game/Blueprints/Gameplay/BP_Player.SetHoldingObject` Player Object)
            (`self.K2_DestroyActor` Object)
            (return false)))))
    (:`False`
      (goto _label))))

(fn `UserConstructionScript`
  (`parent.UserConstructionScript`))