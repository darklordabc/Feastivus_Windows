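; A stack actor that holds objects piled vertically, which a free player picks up from the top when the stack is available.
; Objects attach to the trigger box at index-based height offsets, packed on construction and BeginPlay or added uniquely at runtime.
; Each object is notified when stacked or removed, via Feastivus attach and detach helpers.
; When removal leaves one object, that object replaces the stack, which destroys itself.
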(event `self.ReceiveBeginPlay`
  (`parent.ReceiveBeginPlay`)
  (`self.PackObjects`))

(fn `AddObject`
  (params (Object :type "/Game/Blueprints/Gameplay/BP_DynamicObject Object Reference"))
  (bind _returnvalue (`KismetArrayLibrary.Array_AddUnique` (`self.Objects`) Object))
  (if (`KismetArrayLibrary.Array_IsValidIndex` (`self.Objects`) _returnvalue)
    (bind _attachedobject (`/Game/Blueprints/BPFL_FeastivusAPI.FeastivusAttach` Object (`self.TriggerBox`)))
    (`self.K2_SetActorRelativeLocation` _attachedobject (`KismetMathLibrary.MakeVector` 0.0 0.0 (* _returnvalue (`self.VerticalOffset`))) false true)
    (message `/Game/Blueprints/Gameplay/Tools/BPI_Stackable.OnStacked` _attachedobject self)
    (return)
    (else
      (return))))

(fn `InteractWith`
  (params (Object :type "/Game/Blueprints/Gameplay/BP_DynamicObject Object Reference") (Player :type "/Game/Blueprints/Gameplay/BP_Player Object Reference"))
  (returns (bStartProcessing :type Boolean) (bSuccess :type Boolean))
  (bind _free (`/Game/Blueprints/Gameplay/BP_Player.IsFree` Player))
  (if (and (`self.bAvailableToPickup`) _free)
    (bind _detachedobject (`self.RemoveObject` (`KismetArrayLibrary.Array_LastIndex` (`self.Objects`))))
    (bind _success (`/Game/Blueprints/Gameplay/BP_Player.SetHoldingObject` Player _detachedobject))
    (return false _success)
    (else
      (return false false))))

(fn `PackObjects`
  (for (_array_element _array_index) (`self.Objects`)
    (bind _attachedobject (`/Game/Blueprints/BPFL_FeastivusAPI.FeastivusAttach` _array_element (`self.TriggerBox`)))
    (`self.K2_SetActorRelativeLocation` _attachedobject (`KismetMathLibrary.MakeVector` 0.0 0.0 (* _array_index (`self.VerticalOffset`))) false true)
    (message `/Game/Blueprints/Gameplay/Tools/BPI_Stackable.OnStacked` _attachedobject self)))

(fn `RemoveObject`
  (params (Index :type Integer))
  (returns (DetachedObject :type "/Game/Blueprints/Gameplay/BP_DynamicObject Object Reference"))
  (bind _detachedobject (`/Game/Blueprints/BPFL_FeastivusAPI.FeastivusDetach` (`|GetArrayItem` (`self.Objects`) Index)))
  (message `/Game/Blueprints/Gameplay/Tools/BPI_Stackable.OnRemovedFromStack` _detachedobject self)
  (`KismetArrayLibrary.Array_Remove` (`self.Objects`) Index)
  (if (== (`KismetArrayLibrary.Array_Length` (`self.Objects`)) 1)
    (bind _detachedobject_2 (`self.RemoveObject` 0))
    (`/Game/Blueprints/BPFL_FeastivusAPI.FeastivusReplaceObject` self _detachedobject_2)
    (`self.K2_DestroyActor`))
  (return _detachedobject))

(fn `UserConstructionScript`
  (`parent.UserConstructionScript`)
  (`self.PackObjects`))