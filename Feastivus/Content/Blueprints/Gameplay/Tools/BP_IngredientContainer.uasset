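; BP_IngredientContainer is a tool actor that holds ingredient actors up to its slot count and shows their icons on a 2x2 layout widget.
; BeginPlay enables the widget's slots to match that count.
; TakeIngredient rejects duplicates or overflow, otherwise adds the ingredient and uses its array index as the icon's slot.
; DestroyAllIngredients destroys the held actors, empties the array and clears the widget.
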(event `self.ReceiveBeginPlay`
  (`parent.ReceiveBeginPlay`)
  (bind _asbpw_icon_layout_2x2 (`self.GetLayoutWidget`))
  (`/Game/Blueprints/Widgets/BPW_IconLayout2x2.SetEnabledSlots` _asbpw_icon_layout_2x2 (`self.Slots`)))

(event `Event Set Layout Widget Icon`
  (params (IconTexture :type "Texture2D Object Reference") (Slot :type Integer))
  (bind _asbpw_icon_layout_2x2 (`self.GetLayoutWidget`))
  (`/Game/Blueprints/Widgets/BPW_IconLayout2x2.SetSlotIconTexture` _asbpw_icon_layout_2x2 IconTexture Slot))

(event `Event Clear Layout Widget`
  (bind _asbpw_icon_layout_2x2 (`self.GetLayoutWidget`))
  (`/Game/Blueprints/Widgets/BPW_IconLayout2x2.ClearAllSlots` _asbpw_icon_layout_2x2))

(fn `DestroyAllIngredients`
  (`/Game/Blueprints/BPFL_FeastivusAPI.FeastivusDestroyArrayOfActors` (`self.Ingredients`))
  (`KismetArrayLibrary.Array_Clear` (`self.Ingredients`))
  (`self.Event Clear Layout Widget`))

(fn `GetAllIngredients`
  (returns (Ingredients :type "Array of /Game/Blueprints/Gameplay/Ingredients/BP_Ingredient Object Reference"))
  (return (`self.Ingredients`)))

(fn `TakeIngredient`
  (params (Ingredient :type "/Game/Blueprints/Gameplay/Ingredients/BP_Ingredient Object Reference"))
  (returns (Success :type Boolean))
  (locals (IsSuccess :type Boolean))
  (bind _output_get (set `local.IsSuccess` (and (> (`self.Slots`) (`KismetArrayLibrary.Array_Length` (`self.Ingredients`))) (not (`KismetArrayLibrary.Array_Contains` (`self.Ingredients`) Ingredient)))))
  (if _output_get
    (bind _returnvalue (`KismetArrayLibrary.Array_AddUnique` (`self.Ingredients`) Ingredient))
    (`self.Event Set Layout Widget Icon` (`.IconTexture_4_8E1524674FDD5ABEE7D6ECABD6ADFE62` (break `/Game/Blueprints/Gameplay/S_ObjectUIInfo` (`/Game/Blueprints/Gameplay/Ingredients/BP_Ingredient.UIInfo` Ingredient))) _returnvalue))
  (return (`local.IsSuccess`)))

(fn `UserConstructionScript`
  (`parent.UserConstructionScript`))