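; Player controller that puts a recipe order list on screen for the player.
; On BeginPlay, only the non-authority (Remote) side creates the BPW_OrderList widget and adds it to the viewport.
; It then feeds three hardcoded salad rows from DT_Recipes into AddOrder on staggered delays, each lookup running only if the previous row was found.
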(event `self.ReceiveBeginPlay`
  (`/Engine/EditorBlueprintResources/ActorMacros.Switch Has Authority`
    (:`Remote`
      (bind _returnvalue (`|CreateWidget` "/Game/Blueprints/Widgets/BPW_OrderList.BPW_OrderList_C" self))
      (`UserWidget.AddToViewport` _returnvalue 0)
      (`KismetSystemLibrary.Delay` 1.5)
      (bind _returnvalue_2 (`|GetDataTableRow` "/Game/Recipes/DT_Recipes.DT_Recipes" "MangoSalad")
        (:`then`
          (`/Game/Blueprints/Widgets/BPW_OrderList.AddOrder` _returnvalue _returnvalue_2)
          (`KismetSystemLibrary.Delay` 1.5)
          (bind _returnvalue_3 (`|GetDataTableRow` "/Game/Recipes/DT_Recipes.DT_Recipes" "MixedTangoSalad")
            (:`then`
              (`/Game/Blueprints/Widgets/BPW_OrderList.AddOrder` _returnvalue _returnvalue_3)
              (`KismetSystemLibrary.Delay` 1.5)
              (bind _returnvalue_4 (`|GetDataTableRow` "/Game/Recipes/DT_Recipes.DT_Recipes" "MixedMangoSalad")
                (:`then`
                  (`/Game/Blueprints/Widgets/BPW_OrderList.AddOrder` _returnvalue _returnvalue_4))))))))))

(fn `UserConstructionScript`)